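; Title menu controller, likely the game instance, that manages the index, host and server list screens and multiplayer session hosting and browsing.
; Page events create their widgets or reshow existing ones, with back events restoring the index page.
; Hosting creates a session and opens the third-person example map as a listen server.
; Refreshing clears the server list and searches sessions, using a Steam checkbox to choose LAN, to create row widgets.
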(event Custom|lauchTitleMenu
  (bind _returnvalue (Game|GetPlayerController 0))
  ;[1 1 1] IndePage Controlls
  (Utilities|IsValid (Variables|Default|GetIndexPage)
    (:Is%20Valid
      _)
    (:Is%20Not%20Valid
      (bind _returnvalue_2 (UserInterface|CreateWidget "/Game/HUD/IndexPage.IndexPage_C" _returnvalue))
      (bind _output_get (Variables|Default|SetIndexPage _returnvalue_2))))
  (UserInterface|Viewport|AddtoViewport _output_get 0)
  (Variables|/Script/Engine.PlayerController|SetbShowMouseCursor _returnvalue true)
  (Input|SetInputModeGameandUI _returnvalue _returnvalue_2 "DoNotLock" true))

(event Custom|LauchHostPage
  ;[1 1 1] HostPage Controlls
  (Utilities|IsValid (Variables|Default|GetHostPage)
    (:Is%20Valid
      (Widget|SetVisibility (Variables|Default|GetHostPage) "Visible"))
    (:Is%20Not%20Valid
      (bind _returnvalue (UserInterface|CreateWidget "/Game/HUD/HostPage.HostPage_C" (Game|GetPlayerController 0)))
      (bind _output_get (Variables|Default|SetHostPage _returnvalue))
      (UserInterface|Viewport|AddtoViewport _output_get 0))))

(event Custom|HostEvnt
  (bind (_returnvalue _steamenabled) (Utilities|SteamHost?))
  ;[1 1 1] HostPage Controlls
  (|Session _returnvalue 20 _steamenabled
    (:OnSuccess
      (Game|OpenLevel(byName) "ThirdPersonExampleMap" true "Listen")
      (Input|SetInputModeGameOnly _returnvalue))
    (:OnFailure
      (Development|PrintString "failed to host the game"))))

(event Custom|ServerListUpdate
  ;[1 1 1] ServerListPage contrills
  (CallFunction|ClearServersList)
  (Utilities|ShowSessionsFound))

(event Custom|BackBtnEvtHostPage
  ;[1 1 1] HostPage Controlls
  (Widget|SetVisibility (Variables|Default|GetIndexPage) "Visible"))

(event Custom|backBtnEvntServerPage
  ;[1 1 1] ServerListPage contrills
  (Widget|SetVisibility (Variables|Default|GetIndexPage) "Visible"))

(event Custom|LaunchServerPage
  ;[1 1 1] ServerListPage contrills
  (Utilities|IsValid (Variables|Default|GetServerPage)
    (:Is%20Valid
      (Widget|SetVisibility (Variables|Default|GetServerPage) "Visible"))
    (:Is%20Not%20Valid
      (bind _returnvalue (UserInterface|CreateWidget "/Game/HUD/ServerList.ServerList_C" (Game|GetPlayerController 0)))
      (bind _output_get (Variables|Default|SetServerPage _returnvalue))
      (UserInterface|Viewport|AddtoViewport _output_get 0))))

(fn ClearServersList
  (Widget|Panel|ClearChildren (Variables|/Game/HUD/ServerList.ServerList_C|GetServerList (Variables|Default|GetServerPage))))